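; Enemy Blueprint that takes damage, shows its health on a widget and dies when HP runs out.
; AnyDamage subtracts from HP, then plays a head-hit montage and passes HP to the widget through UpdateWidgetUI.
; A DoOnce resets only while HP stays positive, so later hits skip these reactions.
; At zero or below, it plays a sound and stunned animation, then destroys itself after a delay.
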(event Collision|EventActorBeginOverlap
  (params (OtherActor :type Actor%20Object%20Reference)))

(event EventTick
  (params (DeltaSeconds :type Float%20%28single-precision%29)))

(event Game|Damage|EventAnyDamage
  (params (Damage :type Float%20%28single-precision%29) (DamageType :type Damage%20Type%20Object%20Reference) (InstigatedBy :type Controller%20Object%20Reference) (DamageCauser :type Actor%20Object%20Reference))
  (bind _output_get (Variables|Default|SetHP (- (Variables|Default|GetHP) Damage)))
  (Utilities|FlowControl|DoOnce false :!label _label
    (:Completed
      (Animation|PlayAnimMontage "/Game/Enemy/Anim/Animations/Big_Hit_To_Head_Montage.Big_Hit_To_Head_Montage" 1.0 "None")
      (Utilities|UpdateWidgetUI)
      (if (<= _output_get 0.0)
        (Utilities|FlowControl|DoOnce false
          (:Completed
            (Audio|PlaySound2D "/Game/Enemy/Audio/aaaaaaa.aaaaaaa" 1.0 1.0 0.0 0 0)
            (Components|Animation|PlayAnimation (Variables|Character|GetMesh) "/Game/Enemy/Anim/Animations/Stunned.Stunned" false)
            (Utilities|FlowControl|Delay 5.0)
            (Actor|DestroyActor)))
        (else
          (goto _label Reset))))))

(fn ConstructionScript)